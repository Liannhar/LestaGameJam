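; BP_Ded is the pawn that walks a point-to-point path during the game's active phase.
; It looks up each Path entry in the current point's ReachablePoints, rotates, then moves by timeline at distance-scaled speed, calling BPStepComponent on arrival.
; Overlapping Lyja slides it onto Lyja, while BP_CAT slides it back to the previous point, both with a sound.
; Finishing the path or either slide starts the game mode's passive phase.
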(event OnComponentBeginOverlap(Ded_Capsule)
  (params (OverlappedComponent :type Primitive%20Component%20Object%20Reference) (OtherActor :type Actor%20Object%20Reference) (OtherComp :type Primitive%20Component%20Object%20Reference) (OtherBodyIndex :type Integer) (bFromSweep :type Boolean) (SweepResult :type Hit%20Result%20Structure%20%28by%20ref%29))
  (bind _returnvalue (Transformation|GetActorLocation))
  (bind _returnvalue_2 (Transformation|GetActorLocation))
  (bind _previuos_point (Variables|Default|GetPreviuos%20Point))
  (bind _returnvalue_3 (Transformation|GetActorLocation _previuos_point))
  (Utilities|FlowControl|Sequence
    (:then_0
      (bind _aslyja (Utilities|Casting|CastToLyja OtherActor))
      (Variables|Default|SetLyja_Ref _aslyja)
      (Audio|PlaySound2D "/Game/Sounds/Crehtit_Cue.Crehtit_Cue" 1.0 1.0 0.0 0 0)
      (bind _clamp (Timeline|Timeline_2 PlayFromStart)
        (:Update
          (bind _output_get (Variables|Default|SetCurrentLocation (Math|Vector|MakeVector (.x _returnvalue_2) (.y _returnvalue_2) (.z _returnvalue_2))))
          (Transformation|SetActorLocation (Math|Vector|Lerp(Vector) _output_get (Math|Vector|MakeVector (.x (Transformation|GetActorLocation (Variables|Default|GetLyja_Ref))) (.y (Transformation|GetActorLocation (Variables|Default|GetLyja_Ref))) (.z _returnvalue_2)) _clamp) true false))
        (:Finished
          (Class|LestaGameJamGameModeBase|StartPassivePhase (Variables|Default|GetGameMode))
          (Variables|Default|SetPathIndex 0))))
    (:then_1
      (bind _asbp_cat (Utilities|Casting|CastToBP_CAT OtherActor))
      (Variables|Default|SetCAT_Ref _asbp_cat)
      (Audio|PlaySound2D "/Game/Sounds/Crehtit_Cue.Crehtit_Cue" 1.0 1.0 0.0 0 0)
      (bind _clamp_2 (Timeline|Timeline_0 PlayFromStart)
        (:Update
          (bind _output_get_2 (Variables|Default|SetCurrentLocation (Math|Vector|MakeVector (.x _returnvalue) (.y _returnvalue) (.z _returnvalue))))
          (Transformation|SetActorLocation (Math|Vector|Lerp(Vector) _output_get_2 (Math|Vector|MakeVector (.x _returnvalue_3) (.y _returnvalue_3) (.z _returnvalue)) _clamp_2) true false))
        (:Finished
          (Class|LestaGameJamGameModeBase|StartPassivePhase (Variables|Default|GetGameMode))
          (Variables|Default|SetPathIndex 0))))))

(event Custom|OnActivePhase_Event
  (CallFunction|MoveAlongthePath1)
  (Utilities|Casting|CastToBP_GJPlayerController (Pawn|GetController)))

(event Custom|Stop_Walk
  (bind _clamp (Timeline|Timeline_1 Stop)
    (:Update
      (Transformation|SetActorLocation (Math|Vector|Lerp(Vector) (Variables|Default|GetCurrentLocation) (Transformation|GetActorLocation (Variables|Default|GetNextPoint)) _clamp) true false))
    (:Finished
      (Variables|Default|SetCurrentPoint (Variables|Default|GetNextPoint))
      (Variables|Default|SetCurrentLocation (Transformation|GetActorLocation))
      (CallFunction|StopMoving)
      (bind _result (Math|Integer|IncrementInt (Variables|Default|GetPathIndex))
        (:%20%20
          (Variables|Default|SetRotation (.yaw (Transformation|GetActorRotation)))
          (Default|Step (Variables|Default|GetBP_Step_Component))
          (if (>= _result (Variables|Default|GetPathLength))
            (Class|LestaGameJamGameModeBase|StartPassivePhase (Variables|Default|GetGameMode))
            (Variables|Default|SetPathIndex 0)
            (elif (.ReturnValue (Utilities|Map|Find (Variables|/Game/BP_Point.BP_Point_C|GetReachablePoints (Variables|Default|GetCurrentPoint)) (Utilities|Array|Get(acopy) (Variables|Default|GetPath) (Variables|Default|GetPathIndex))))
              (Variables|Default|SetPreviuos%20Point (Variables|Default|GetCurrentPoint))
              (Variables|Default|SetNextPoint (.Value (Utilities|Map|Find (Variables|/Game/BP_Point.BP_Point_C|GetReachablePoints (Variables|Default|GetCurrentPoint)) (Utilities|Array|Get(acopy) (Variables|Default|GetPath) (Variables|Default|GetPathIndex)))))
              (CallFunction|StartMoving)
              (Components|Timeline|SetPlayRate (Variables|Default|GetTimeline_1) (/ 1.0 (/ (Math|Vector|Distance(Vector) (Variables|Default|GetCurrentLocation) (Transformation|GetActorLocation (Variables|Default|GetNextPoint))) 6e+02)))
              (|Rotate
                (:PlayFromStart
                  (Timeline|Timeline_1 PlayFromStart))))))))))

(event Custom|Stop_moving
  (Variables|Default|SetIs_Moving false))

(event Custom|Start_moving
  (Variables|Default|SetIs_Moving true))

(event Custom|MoveAlongThePath_1
  (Variables|Default|SetCurrentLocation (Transformation|GetActorLocation))
  (Variables|Default|SetPathLength (Utilities|Array|Length (Variables|Default|GetPath)))
  (if (.ReturnValue (Utilities|Map|Find (Variables|/Game/BP_Point.BP_Point_C|GetReachablePoints (Variables|Default|GetCurrentPoint)) (Utilities|Array|Get(acopy) (Variables|Default|GetPath) (Variables|Default|GetPathIndex)))) :!label _label
    (Variables|Default|SetPreviuos%20Point (Variables|Default|GetCurrentPoint))
    (Variables|Default|SetNextPoint (.Value (Utilities|Map|Find (Variables|/Game/BP_Point.BP_Point_C|GetReachablePoints (Variables|Default|GetCurrentPoint)) (Utilities|Array|Get(acopy) (Variables|Default|GetPath) (Variables|Default|GetPathIndex)))))
    (CallFunction|StartMoving)
    (Components|Timeline|SetPlayRate (Variables|Default|GetTimeline_1) (/ 1.0 (/ (Math|Vector|Distance(Vector) (Variables|Default|GetCurrentLocation) (Transformation|GetActorLocation (Variables|Default|GetNextPoint))) 6e+02)))
    (|Rotate
      (:PlayFromStart
        (bind _clamp (Timeline|Timeline_1 PlayFromStart)
          (:Update
            (Transformation|SetActorLocation (Math|Vector|Lerp(Vector) (Variables|Default|GetCurrentLocation) (Transformation|GetActorLocation (Variables|Default|GetNextPoint)) _clamp) true false))
          (:Finished
            (Variables|Default|SetCurrentPoint (Variables|Default|GetNextPoint))
            (Variables|Default|SetCurrentLocation (Transformation|GetActorLocation))
            (CallFunction|StopMoving)
            (bind _result (Math|Integer|IncrementInt (Variables|Default|GetPathIndex))
              (:%20%20
                (Variables|Default|SetRotation (.yaw (Transformation|GetActorRotation)))
                (Default|Step (Variables|Default|GetBP_Step_Component))
                (if (>= _result (Variables|Default|GetPathLength))
                  (Class|LestaGameJamGameModeBase|StartPassivePhase (Variables|Default|GetGameMode))
                  (Variables|Default|SetPathIndex 0)
                  (else
                    (goto _label)))))))))))

(event EventBeginPlay
  (bind _returnvalue (Actor|GetActorOfClass "/Game/Lyja/Lyja.Lyja_C"))
  (Variables|Default|SetLyja_Ref _returnvalue)
  (Transformation|SetActorLocation (Transformation|GetActorLocation (Variables|Default|GetCurrentPoint)) false false)
  (bind _aslesta_game_jam_game_mode_base (Utilities|Casting|CastToLestaGameJamGameModeBase (Game|GetGameMode)))
  (bind _output_get (Variables|Default|SetGameMode _aslesta_game_jam_game_mode_base))
  (EventDispatchers|AssignOnActivePhase _output_get (delegate Custom|OnActivePhase_Event))
  (Audio|PlaySound2D "/Game/Sounds/What_Is_Love_Cue.What_Is_Love_Cue" 1.0 1.0 0.0 0 0))

(fn ConstructionScript
  (|CallParentFunction))