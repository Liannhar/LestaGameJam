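; Base pawn Blueprint that travels a predefined route through linked points.
; MoveAlongThePath resolves each Path entry through the current point's ReachablePoints map to get the next point actor.
; The Moving timeline lerps the pawn there with sweep, then updates CurrentPoint and replays until the path ends.
; BeginPlay is empty, and the snap-to-start and movement call nodes are disconnected, so this graph never starts movement itself.
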(event Custom|MoveAlongThePath
  ;[1 1 1] Событие, которое отвечает за перемещение объекта по заранее заданному маршруту
  (Variables|Movement|SetCurrentLocation (Transformation|GetActorLocation))
  (Variables|Movement|SetPathLength (Utilities|Array|Length (Variables|Movement|GetPath)))
  (Variables|Movement|SetNextPoint (.Value (Utilities|Map|Find (Variables|/Game/Blueprints/Akhmad/BP_Point.BP_Point_C|GetReachablePoints (Variables|Movement|GetCurrentPoint)) (Utilities|Array|Get(acopy) (Variables|Movement|GetPath)))))
  (bind _clamp (Timeline|Moving Play)
    (:Update
      (Transformation|SetActorLocation (Math|Vector|Lerp(Vector) (Variables|Movement|GetCurrentLocation) (Transformation|GetActorLocation (Variables|Movement|GetNextPoint)) _clamp) true false))
    (:Finished
      (Variables|Movement|SetCurrentPoint (Variables|Movement|GetNextPoint))
      (Variables|Movement|SetCurrentLocation (Transformation|GetActorLocation))
      (bind _result (Math|Integer|IncrementInt (Variables|Movement|GetPathIndex))
        (:%20%20
          (if (not (>= _result (Variables|Movement|GetPathLength)))
            (Variables|Movement|SetNextPoint (.Value (Utilities|Map|Find (Variables|/Game/Blueprints/Akhmad/BP_Point.BP_Point_C|GetReachablePoints (Variables|Movement|GetCurrentPoint)) (Utilities|Array|Get(acopy) (Variables|Movement|GetPath) (Variables|Movement|GetPathIndex)))))
            (Timeline|Moving PlayFromStart)))))))

(event EventBeginPlay)

(fn ConstructionScript)