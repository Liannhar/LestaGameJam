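; BP_Health_Component is a component that tracks its owner's health and ends the game when it runs out.
; Health is set to a fixed starting value on BeginPlay and polled every Tick.
; Once it reaches zero or below, a DoOnce fires Death, which casts the game mode to BP_LestaGameJamGameModeBase and calls GameOver.
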(event Custom|Death
  (bind _asbp_lesta_game_jam_game_mode_base (Utilities|Casting|CastToBP_LestaGameJamGameModeBase (Game|GetGameMode)))
  (Class|LestaGameJamGameModeBase|GameOver _asbp_lesta_game_jam_game_mode_base))

(event EventBeginPlay
  (Variables|Default|SetHealth 3.0))

(event EventTick
  (params (DeltaSeconds :type Float%20%28single-precision%29))
  (if (<= (Variables|Default|GetHealth) 0.0)
    (Utilities|FlowControl|DoOnce false
      (:Completed
        (CallFunction|Death)))))