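; BP_Point is a waypoint actor that detects when the BP_Ded actor steps on it and can validate paths through linked points.
; When Ded's capsule overlaps its box, it passes itself to PointArray on BP_Ded_Inst, the game instance, and sets DedStep.
; CheckIfPathReachable recursively follows the ReachablePoints map, consuming one path entry per point and failing on a missing link.
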(event OnComponentBeginOverlap(Box)
  (params (OverlappedComponent :type Primitive%20Component%20Object%20Reference) (OtherActor :type Actor%20Object%20Reference) (OtherComp :type Primitive%20Component%20Object%20Reference) (OtherBodyIndex :type Integer) (bFromSweep :type Boolean) (SweepResult :type Hit%20Result%20Structure%20%28by%20ref%29))
  (if (== OtherComp (Variables|/Game/Ded/BP_Ded.BP_Ded_C|GetDed_Capsule (Variables|Default|GetDed_Ref)))
    (Default|PointArray (.AsBP%20Ded%20Inst (Utilities|Casting|CastToBP_Ded_Inst (Game|GetGameInstance))) self)
    (Variables|Default|SetDed_Step true)))

(event EventBeginPlay
  (bind _returnvalue (Actor|GetActorOfClass "/Game/Ded/BP_Ded.BP_Ded_C"))
  (Variables|Default|SetDed_Ref _returnvalue))

(fn ConstructionScript)

(fn CheckifPathReachable
  (params (Path :type Array%20of%20Integers))
  (bind _output_get (LocalVariables|SetLocalPath Path))
  (if (Utilities|Array|IsNotEmpty Path)
    (LocalVariables|SetNextPoint (.Value (Utilities|Map|Find (Variables|Default|GetReachablePoints) (Utilities|Array|Get(acopy) _output_get))))
    (if (.ReturnValue (Utilities|Map|Find (Variables|Default|GetReachablePoints) (Utilities|Array|Get(acopy) _output_get)))
      (Utilities|Array|RemoveIndex (LocalVariables|GetLocalPath))
      (bind _pathreachable (CallFunction|CheckifPathReachable (LocalVariables|GetNextPoint) (LocalVariables|GetLocalPath)))
      (return _pathreachable)
      (else
        (return false)))
    (else
      (return true))))