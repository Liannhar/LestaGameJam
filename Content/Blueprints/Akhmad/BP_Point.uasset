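; BP_Point is a node in a linked point graph that tests whether a given path can be followed from it.
; CheckIfPathReachable looks up the first path entry in the ReachablePoints map, removes it, then recurses on the mapped point with the remaining path.
; A failed lookup returns false; the function has no explicit empty-path check or branch that returns true.
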(fn ConstructionScript)

(fn CheckifPathReachable
  (params (Path :type Array%20of%20Integers))
  (bind _output (Utilities|Array|Get(acopy) Path))
  (bind _reachablepoints (Variables|Default|GetReachablePoints))
  (bind (_value _returnvalue) (Utilities|Map|Find _reachablepoints _output))
  (LocalVariables|SetNextPoint _value)
  (if _returnvalue
    (Utilities|Array|RemoveIndex Path)
    (bind _pathreachable (CallFunction|CheckifPathReachable (LocalVariables|GetNextPoint) Path))
    (return _pathreachable)
    (else
      (return false))))