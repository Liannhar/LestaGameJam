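; Cat actor that acts as a hazard for the BP_Ded character, costing it health on contact.
; BeginPlay caches the BP_Ded instance and the LestaGameJam game mode.
; When BP_Ded overlaps the box, the cat halts it, hands it the cat's Path and subtracts one health.
; It then starts hit montages on both without waiting for completion and triggers the game mode's passive phase.
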(event OnComponentBeginOverlap(Box)
  (params (OverlappedComponent :type Primitive%20Component%20Object%20Reference) (OtherActor :type Actor%20Object%20Reference) (OtherComp :type Primitive%20Component%20Object%20Reference) (OtherBodyIndex :type Integer) (bFromSweep :type Boolean) (SweepResult :type Hit%20Result%20Structure%20%28by%20ref%29))
  (bind _ded_ref (Variables|Default|GetDed_Ref))
  (bind _ded_ref_2 (Variables|Default|GetDed_Ref))
  (bind _bp_health_component (Variables|/Game/Blueprints/Akhmad/Ded/BP_Ded.BP_Ded_C|GetBP_Health_Component _ded_ref))
  (if (== OtherActor (Variables|Default|GetDed_Ref))
    (Default|StopWalk _ded_ref_2)
    (Default|StopMoving _ded_ref_2)
    (Variables|/Game/Blueprints/Akhmad/BP_PawnBase.BP_PawnBase_C|SetPath _ded_ref_2 (Variables|Default|GetPath))
    (Variables|/Game/Blueprints/Akhmad/Ded/BP_Health_Component.BP_Health_Component_C|SetHealth _bp_health_component (- (Variables|/Game/Blueprints/Akhmad/Ded/BP_Health_Component.BP_Health_Component_C|GetHealth _bp_health_component) 1.0))
    (Animation|Montage|PlayMontage (Variables|/Game/Blueprints/Akhmad/BP_PawnBase.BP_PawnBase_C|GetSkeletalMesh _ded_ref) "/Game/Blueprints/Akhmad/Animations/Ded_Hit_Montage.Ded_Hit_Montage" 1.5
      (:then
        (Animation|Montage|PlayMontage (Variables|Default|GetCAT) "/Game/Blueprints/Akhmad/Cat/Cat_Hit_Montage.Cat_Hit_Montage"
          (:then
            (Class|LestaGameJamGameModeBase|StartPassivePhase (Variables|Default|GetGameMode))))))))

(event EventBeginPlay
  (bind _returnvalue (Actor|GetActorOfClass "/Game/Blueprints/Akhmad/Ded/BP_Ded.BP_Ded_C"))
  (Variables|Default|SetDed_Ref _returnvalue)
  (bind _aslesta_game_jam_game_mode_base (Utilities|Casting|CastToLestaGameJamGameModeBase (Game|GetGameMode)))
  (Variables|Default|SetGameMode _aslesta_game_jam_game_mode_base))

(event Collision|EventActorBeginOverlap
  (params (OtherActor :type Actor%20Object%20Reference)))

(event EventTick
  (params (DeltaSeconds :type Float%20%28single-precision%29)))

(fn ConstructionScript)