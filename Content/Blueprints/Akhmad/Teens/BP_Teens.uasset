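; BP_Teens is a teen NPC with a random material that roams a waypoint graph and harms the old man character, BP_Ded.
; The game mode's active phase starts movement, with next points drawn from reachable points using BP_Teen_Controller's path and a weighted check.
; Timelines turn and move it at distance-scaled rates, starting each hop only while BP_Ded moves.
; Overlapping BP_Ded's capsule costs him health, plays hit and angry montages, and stops the teen.
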(event OnComponentBeginOverlap(Teen_Capsule)
  (params (OverlappedComponent :type Primitive%20Component%20Object%20Reference) (OtherActor :type Actor%20Object%20Reference) (OtherComp :type Primitive%20Component%20Object%20Reference) (OtherBodyIndex :type Integer) (bFromSweep :type Boolean) (SweepResult :type Hit%20Result%20Structure%20%28by%20ref%29))
  (bind _ded_ref (Variables|Default|GetDed_Ref))
  (bind _bp_health_component (Variables|/Game/Blueprints/Akhmad/Ded/BP_Ded.BP_Ded_C|GetBP_Health_Component _ded_ref))
  (bind _asbp_ded (Utilities|Casting|CastToBP_Ded OtherActor))
  (if (== OtherComp (Variables|/Game/Blueprints/Akhmad/Ded/BP_Ded.BP_Ded_C|GetDed_Capsule _asbp_ded))
    (Utilities|FlowControl|DoOnce false
      (:Completed
        (Variables|/Game/Blueprints/Akhmad/Ded/BP_Health_Component.BP_Health_Component_C|SetHealth _bp_health_component (- (Variables|/Game/Blueprints/Akhmad/Ded/BP_Health_Component.BP_Health_Component_C|GetHealth _bp_health_component) 1.0))
        (Animation|Montage|PlayMontage (Variables|/Game/Blueprints/Akhmad/BP_PawnBase.BP_PawnBase_C|GetSkeletalMesh _ded_ref) "/Game/Blueprints/Akhmad/Animations/Ded_Hit_Montage.Ded_Hit_Montage" 1.5
          (:then
            (Animation|Montage|PlayMontage (Variables|Default|GetSkeletalMesh) "/Game/Blueprints/Akhmad/Teens/Angry_Gesture_Montage.Angry_Gesture_Montage" 1.5
              (:then
                (CallFunction|StopGo)
                (CallFunction|StopMoving)
                (CallFunction|Reset)))))))))

(event Custom|OnActivePhase_Event
  (CallFunction|MoveAlongthePath))

(event Custom|Stop_go
  (bind _clamp (Timeline|Timeline_0_0 Stop)
    (:Update
      (Transformation|SetActorLocation (Math|Vector|Lerp(Vector) (Variables|Default|GetCurrentLocation) (Transformation|GetActorLocation (Variables|Default|GetNextPoint)) _clamp) true false))
    (:Finished
      (Variables|Default|SetCurrentPoint (Variables|Default|GetNextPoint))
      (Variables|Default|SetCurrentLocation (Transformation|GetActorLocation))
      (CallFunction|StopMoving)
      (if (.ReturnValue (Utilities|Map|Find (Variables|/Game/Blueprints/Akhmad/BP_Point.BP_Point_C|GetReachablePoints (Variables|Default|GetCurrentPoint)) (Variables|/Game/Blueprints/Akhmad/Teens/BP_Teen_Controller.BP_Teen_Controller_C|GetPath (Variables|Default|GetBP_TC))))
        (bind _find (CallFunction|RandomPath (.Value (Utilities|Map|Find (Variables|/Game/Blueprints/Akhmad/BP_Point.BP_Point_C|GetReachablePoints (Variables|Default|GetCurrentPoint)) (Variables|/Game/Blueprints/Akhmad/Teens/BP_Teen_Controller.BP_Teen_Controller_C|GetPath (Variables|Default|GetBP_TC))))))
        (Variables|Default|SetNextPoint _find)
        (if (Variables|/Game/Blueprints/Akhmad/Ded/BP_Ded.BP_Ded_C|GetIs_Moving (Variables|Default|GetDed_Ref))
          (Components|Timeline|SetPlayRate (Variables|Default|GetTimeline_0_0) (/ 1.0 (/ (Math|Vector|Distance(Vector) (Variables|Default|GetCurrentLocation) (Transformation|GetActorLocation (Variables|Default|GetNextPoint))) 6.5e+02)))
          (CallFunction|StartMoving)
          (|Rotate_2
            (:PlayFromStart
              (Timeline|Timeline_0_0 PlayFromStart)))
          (else
            (Timeline|Timeline_0_0 Stop)))
        (else
          (Utilities|FlowControl|Delay 0.2)
          (CallFunction|Refind))))))

(event Custom|Stop_moving
  (Variables|Default|SetIs_Walking false))

(event Custom|Start_moving
  (Variables|Default|SetIs_Walking true))

(event Custom|Reset
  (bind _ded_ref (Variables|Default|GetDed_Ref))
  (bind _bp_health_component (Variables|/Game/Blueprints/Akhmad/Ded/BP_Ded.BP_Ded_C|GetBP_Health_Component _ded_ref))
  (Utilities|FlowControl|DoOnce false) ; enters at Reset
)

(event Custom|Refind
  (Default|ResetPoint (Variables|Default|GetBP_TC))
  (if (.ReturnValue (Utilities|Map|Find (Variables|/Game/Blueprints/Akhmad/BP_Point.BP_Point_C|GetReachablePoints (Variables|Default|GetCurrentPoint)) (Variables|/Game/Blueprints/Akhmad/Teens/BP_Teen_Controller.BP_Teen_Controller_C|GetPath (Variables|Default|GetBP_TC)))) :!label _label
    (bind _find (CallFunction|RandomPath (.Value (Utilities|Map|Find (Variables|/Game/Blueprints/Akhmad/BP_Point.BP_Point_C|GetReachablePoints (Variables|Default|GetCurrentPoint)) (Variables|/Game/Blueprints/Akhmad/Teens/BP_Teen_Controller.BP_Teen_Controller_C|GetPath (Variables|Default|GetBP_TC))))))
    (Variables|Default|SetNextPoint _find)
    (if (Variables|/Game/Blueprints/Akhmad/Ded/BP_Ded.BP_Ded_C|GetIs_Moving (Variables|Default|GetDed_Ref))
      (Components|Timeline|SetPlayRate (Variables|Default|GetTimeline_0_0) (/ 1.0 (/ (Math|Vector|Distance(Vector) (Variables|Default|GetCurrentLocation) (Transformation|GetActorLocation (Variables|Default|GetNextPoint))) 6.5e+02)))
      (CallFunction|StartMoving)
      (|Rotate_2
        (:PlayFromStart
          (bind _clamp (Timeline|Timeline_0_0 PlayFromStart)
            (:Update
              (Transformation|SetActorLocation (Math|Vector|Lerp(Vector) (Variables|Default|GetCurrentLocation) (Transformation|GetActorLocation (Variables|Default|GetNextPoint)) _clamp) true false))
            (:Finished
              (Variables|Default|SetCurrentPoint (Variables|Default|GetNextPoint))
              (Variables|Default|SetCurrentLocation (Transformation|GetActorLocation))
              (CallFunction|StopMoving)
              (goto _label)))))
      (else
        (Timeline|Timeline_0_0 Stop)))
    (else
      (Utilities|FlowControl|Delay 0.2)
      (CallFunction|Refind))))

(event EventBeginPlay
  (Utilities|FlowControl|Sequence
    (:then_0
      (Transformation|SetActorLocation (Transformation|GetActorLocation (Variables|Default|GetCurrentPoint)) false false)
      (switch int (Math|Random|RandomIntegerinRange 0 2)
        (:0
          (Rendering|Material|SetMaterial (Variables|Default|GetSkeletalMesh) 0 "/Game/Blueprints/Akhmad/Teens/Mat_1/TEEN_M_1.TEEN_M_1"))
        (:1
          (Rendering|Material|SetMaterial (Variables|Default|GetSkeletalMesh) 0 "/Game/Blueprints/Akhmad/Teens/Mat_2/Teen_MAT_2.Teen_MAT_2"))
        (:2
          (Rendering|Material|SetMaterial (Variables|Default|GetSkeletalMesh) 0 "/Game/Blueprints/Akhmad/Teens/Mat_3/Teen_Mat_3.Teen_Mat_3"))))
    (:then_1
      (bind _returnvalue (Actor|GetActorOfClass "/Game/Blueprints/Akhmad/Ded/BP_Ded.BP_Ded_C"))
      (Variables|Default|SetDed_Ref _returnvalue)
      (bind _aslesta_game_jam_game_mode_base (Utilities|Casting|CastToLestaGameJamGameModeBase (Game|GetGameMode)))
      (bind _output_get (Variables|Default|SetGameMode _aslesta_game_jam_game_mode_base))
      (EventDispatchers|AssignOnActivePhase _output_get (delegate Custom|OnActivePhase_Event)))))

(event EventMoveAlongthePath
  (bind _returnvalue (Actor|GetActorOfClass "/Game/Blueprints/Akhmad/Teens/BP_Teen_Controller.BP_Teen_Controller_C"))
  (Variables|Default|SetBP_TC _returnvalue)
  (Variables|Default|SetCurrentLocation (Transformation|GetActorLocation))
  (Variables|Default|SetPathLength (Utilities|Array|Length (Variables|Default|GetPath)))
  (if (.ReturnValue (Utilities|Map|Find (Variables|/Game/Blueprints/Akhmad/BP_Point.BP_Point_C|GetReachablePoints (Variables|Default|GetCurrentPoint)) (Variables|/Game/Blueprints/Akhmad/Teens/BP_Teen_Controller.BP_Teen_Controller_C|GetPath (Variables|Default|GetBP_TC)))) :!label _label
    (bind _find (CallFunction|RandomPath (.Value (Utilities|Map|Find (Variables|/Game/Blueprints/Akhmad/BP_Point.BP_Point_C|GetReachablePoints (Variables|Default|GetCurrentPoint)) (Variables|/Game/Blueprints/Akhmad/Teens/BP_Teen_Controller.BP_Teen_Controller_C|GetPath (Variables|Default|GetBP_TC))))))
    (Variables|Default|SetNextPoint _find)
    (if (Variables|/Game/Blueprints/Akhmad/Ded/BP_Ded.BP_Ded_C|GetIs_Moving (Variables|Default|GetDed_Ref))
      (Components|Timeline|SetPlayRate (Variables|Default|GetTimeline_0_0) (/ 1.0 (/ (Math|Vector|Distance(Vector) (Variables|Default|GetCurrentLocation) (Transformation|GetActorLocation (Variables|Default|GetNextPoint))) 6.5e+02)))
      (CallFunction|StartMoving)
      (|Rotate_2
        (:PlayFromStart
          (bind _clamp (Timeline|Timeline_0_0 PlayFromStart)
            (:Update
              (Transformation|SetActorLocation (Math|Vector|Lerp(Vector) (Variables|Default|GetCurrentLocation) (Transformation|GetActorLocation (Variables|Default|GetNextPoint)) _clamp) true false))
            (:Finished
              (Variables|Default|SetCurrentPoint (Variables|Default|GetNextPoint))
              (Variables|Default|SetCurrentLocation (Transformation|GetActorLocation))
              (CallFunction|StopMoving)
              (goto _label)))))
      (else
        (Timeline|Timeline_0_0 Stop)))
    (else
      (Utilities|FlowControl|Delay 0.2)
      (CallFunction|Refind))))

(fn ConstructionScript
  (|CallParentFunction))

(fn RandomPath
  (params (Point :type BP%20Point%20Object%20Reference))
  (if (Variables|/Game/Blueprints/Akhmad/BP_Point.BP_Point_C|GetDed_Step Point)
    (Variables|Default|SetPoint Point)
    (Variables|Default|SetChance 51.0)
    (if (Math|Random|RandomBoolwithWeight (Variables|Default|GetChance))
      (Default|ResetPoint (Variables|Default|GetBP_TC))
      (return (Variables|Default|GetPoint))
      (else
        (CallFunction|Refind)))
    (else
      (Variables|Default|SetPoint Point)
      (Variables|Default|SetChance 49.0)
      (if (Math|Random|RandomBoolwithWeight (Variables|Default|GetChance))
        (Default|ResetPoint (Variables|Default|GetBP_TC))
        (return (Variables|Default|GetPoint))
        (else
          (CallFunction|Refind))))))