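; BP_Ded_Inst is a Blueprint that counts Ded rounds and clears the DedStep flag on a registered point.
; Point_Array appends points to the Points array, and each Ded_Round call increments StepIndex and checks it.
; Once the count reaches three, it resets to zero, clears DedStep on the first point only and prints that point's name and flag for debugging.
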(event Custom|Reset_Ded_Step
  (bind _points (Variables|Default|GetPoints))
  (bind _output (Utilities|Array|Get(acopy) _points))
  (Variables|Default|SetStep_Index 0)
  (bind _output_get (Variables|/Game/Blueprints/Akhmad/BP_Point.BP_Point_C|SetDed_Step _output false))
  (Development|PrintString (Utilities|GetDisplayName _output))
  (Development|PrintString (Utilities|String|ToString(Boolean) _output_get)))

(event Custom|Check_Step
  (if (>= (Variables|Default|GetStep_Index) 3)
    (CallFunction|ResetDedStep)))

(event Custom|Ded_Round
  (bind _result (Math|Integer|IncrementInt (Variables|Default|GetStep_Index))
    (:%20%20
      (Variables|Default|SetStep_Index _result)
      (CallFunction|CheckStep))))

(event Custom|Point_Array
  (params (NewParam :type BP%20Point%20Object%20Reference))
  (Utilities|Array|Add (Variables|Default|GetPoints) NewParam))