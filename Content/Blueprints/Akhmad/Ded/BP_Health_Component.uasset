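; BP_Health_Component is a health component that ends the game when its Health value runs out.
; BeginPlay sets a small starting Health and caches the first BP_Ded actor found in the level.
; Tick polls Health and, once it reaches zero, uses a DoOnce to fire Death a single time.
; Death calls GameOver on the LestaGameJam game mode, then stops BP_Ded's walking and movement.
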(event Custom|Death
  (bind _ded_ref (Variables|Default|GetDed_Ref))
  (bind _asbp_lesta_game_jam_game_mode_base (Utilities|Casting|CastToBP_LestaGameJamGameModeBase (Game|GetGameMode)))
  (Class|LestaGameJamGameModeBase|GameOver _asbp_lesta_game_jam_game_mode_base)
  (Default|StopWalk _ded_ref)
  (Default|StopMoving _ded_ref))

(event EventBeginPlay
  (Variables|Default|SetHealth 3.0)
  (bind _returnvalue (Actor|GetActorOfClass "/Game/Blueprints/Akhmad/Ded/BP_Ded.BP_Ded_C"))
  (Variables|Default|SetDed_Ref _returnvalue))

(event EventTick
  (params (DeltaSeconds :type Float%20%28single-precision%29))
  (if (<= (Variables|Default|GetHealth) 0.0)
    (Utilities|FlowControl|DoOnce false
      (:Completed
        (CallFunction|Death)))))