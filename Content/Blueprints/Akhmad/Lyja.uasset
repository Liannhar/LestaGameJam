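; Lyja is a hazard actor, named for a puddle, that halts and hurts the BP_Ded character when it touches the hazard's box.
; On BeginPlay it finds and caches the BP_Ded actor in the level.
; When the box begins overlapping that actor's DedCapsule, it calls StopWalk and StopMoving, then directly subtracts a point from the health component's Health.
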(event OnComponentBeginOverlap(Box)
  (params (OverlappedComponent :type Primitive%20Component%20Object%20Reference) (OtherActor :type Actor%20Object%20Reference) (OtherComp :type Primitive%20Component%20Object%20Reference) (OtherBodyIndex :type Integer) (bFromSweep :type Boolean) (SweepResult :type Hit%20Result%20Structure%20%28by%20ref%29))
  (bind _ded_ref (Variables|Components|GetDed_Ref))
  (bind _bp_health_component (Variables|/Game/Blueprints/Akhmad/Ded/BP_Ded.BP_Ded_C|GetBP_Health_Component _ded_ref))
  (if (== OtherComp (Variables|/Game/Blueprints/Akhmad/Ded/BP_Ded.BP_Ded_C|GetDed_Capsule (Variables|Components|GetDed_Ref)))
    (Default|StopWalk _ded_ref)
    (Default|StopMoving _ded_ref)
    (Variables|/Game/Blueprints/Akhmad/Ded/BP_Health_Component.BP_Health_Component_C|SetHealth _bp_health_component (- (Variables|/Game/Blueprints/Akhmad/Ded/BP_Health_Component.BP_Health_Component_C|GetHealth _bp_health_component) 1.0))))

(event EventBeginPlay
  (bind _returnvalue (Actor|GetActorOfClass "/Game/Blueprints/Akhmad/Ded/BP_Ded.BP_Ded_C"))
  (Variables|Components|SetDed_Ref _returnvalue))

(fn ConstructionScript)